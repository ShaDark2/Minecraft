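; BP_Block_Interractible_Chest is an interactable chest block whose lid opens and closes.
; On BeginPlay, after calling the parent, it scales the OpeningChest timeline's play rate by OpenTiming and applies MaterialRef to the locker and lid.
; Each Interract call flip-flops between playing and reversing the timeline, which pitches a pivot scene component between closed and open.
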(event `self.ReceiveBeginPlay`
  ;[1 1 1 1 11] Appelle le BeginPlay parent avant son propre BeginPlay
  (`parent.ReceiveBeginPlay`)
  ;[1 1 1] Set du play rate de l'ouverture du coffre
  (`TimelineComponent.SetPlayRate` (`self.OpeningChest`) (/ 1.0 (`self.OpenTiming`)))
  (`PrimitiveComponent.SetMaterial` (`self.locker`) 0 (`self.materialRef`))
  (`PrimitiveComponent.SetMaterial` (`self.couvercle`) 0 (`self.materialRef`)))

(event `self.Interract`
  ;[1 1 1] Ouverture du coffre
  (`/Engine/EditorBlueprintResources/StandardMacros.FlipFlop`
    (:`A`
      (bind (_direction _rotation) (`Timeline|OpeningChest` :!label _label)
        (:`Update`
          (`SceneComponent.K2_SetRelativeRotation` (`self.Scene`) (`KismetMathLibrary.MakeRotator` 0.0 (`KismetMathLibrary.Lerp` 0.0 -50.0 _rotation)) false false))))
    (:`B`
      (goto _label :!via `Reverse`))))

(fn `UserConstructionScript`
  (`parent.UserConstructionScript`))