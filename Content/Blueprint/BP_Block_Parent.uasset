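; Parent Blueprint for Minecraft-style blocks, handling timed, cancellable breaking and registration in the game's saved block data.
; On BeginPlay it creates a dynamic material, scales the destroy timeline by DestroyTiming, and saves its location and class in GI_Minecraft.
; DestroyBlock drives the material's DestroyAmount through the timeline, then deletes the save entry and destroys the actor.
; StopDestroyBlock halts the timeline and resets DestroyAmount.
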(event `self.ReceiveBeginPlay`
  (bind _cube (`self.Cube`))
  ;[1 1 1] On crée l'instance dynamique du material du block que l'on set dans une variable
  (bind _returnvalue (`PrimitiveComponent.CreateDynamicMaterialInstance` _cube 0 (`PrimitiveComponent.GetMaterial` _cube 0) "None"))
  (set `self.materialRef` _returnvalue)
  ;[1 1 1] Définition du temps de destruction du block
  (`TimelineComponent.SetPlayRate` (`self.DestroyTimeline`) (/ 1.0 (`self.DestroyTiming`)))
  ;[1 1 1 1 14] On récupère le Game Instance "Minecraft" qu'on sauvegarde en variable
  (bind _asgi_minecraft (cast `/Game/Blueprint/GI_Minecraft` (`GameplayStatics.GetGameInstance`)))
  (bind _output_get (set `self.As GI Minecraft` _asgi_minecraft))
  ;[1 1 1] Sauvegarde du block dans le Game Instance
  (`/Game/Blueprint/GI_Minecraft.SaveBlock` _output_get (make `/Game/Blueprint/F_SaveBlock` (`self.K2_GetActorLocation`) (`GameplayStatics.GetObjectClass` self))))

(event `DestroyBlock`
  ;[1 1 1 1 12] Hardcodé dans l'éditeur
  (bind (_direction _alpha) (`Timeline|DestroyTimeline` :`NewTime` (`self.DestroyTiming`) :!via `PlayFromStart` :!label _label)
    (:`Update`
      ;[1 1 1] On modifie la valeur "DestroyAmount" dans le material
      (`MaterialInstanceDynamic.SetScalarParameterValue` (`self.materialRef`) "DestroyAmount" (`KismetMathLibrary.Lerp` 0.0 1.0 _alpha)))
    (:`Finished`
      ;[1 1 1] On supprime le block de la save
      (`/Game/Blueprint/GI_Minecraft.DeleteBlock` (`self.As GI Minecraft`) (make `/Game/Blueprint/F_SaveBlock` (`self.K2_GetActorLocation`) (`GameplayStatics.GetObjectClass` self)))
      ;[1 1 1 1 10] Detruit le block quand la timeline a fini.
      (`self.K2_DestroyActor`))))

(event `StopDestroyBlock`
  ;[1 1 1 1 10] Permet de donner un ordre d'execution
  (`|ExecutionSequence`
    (:`then_0`
      (goto _label :!via `Stop`))
    (:`then_1`
      ;[1 1 1 1 15] Reset la var "DestroyAmount" du material
      (`MaterialInstanceDynamic.SetScalarParameterValue` (`self.materialRef`) "DestroyAmount" 0.0))))

(fn `UserConstructionScript`)