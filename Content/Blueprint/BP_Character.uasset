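; Player character for a Minecraft-style block game, with Enhanced Input movement, sprint, jump, look and a HUD.
; A short camera line trace drives mining, interacting with interactible blocks and placing blocks.
; Mining calls DestroyBlock on the aimed block, and a looping timer rechecks aim to switch or cancel it.
; Placement nudges the hit point along its normal and snaps it to the grid, spawning the block chosen by keys or mouse wheel.
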(event `EnhancedInput|/Game/Blueprint/Inputs/IA_Move`
  (params (ActionValue :type "Vector2D Structure") (ElapsedSeconds :type "Float (double-precision)") (TriggeredSeconds :type "Float (double-precision)") (InputAction :type "InputAction Object Reference" :default "/Game/Blueprint/Inputs/IA_Move.IA_Move"))
  ;[1 1 1] Movement
  ;;[1 1 1] IA_Move
  (:`Triggered`
    (`self.AddMovementInput` (`self.GetActorRightVector`) ActionValue_X)
    (`self.AddMovementInput` (`self.GetActorForwardVector`) ActionValue_Y)))

(event `self.ReceiveBeginPlay`
  ;[1 1 1] BeginPlay
  (`EnhancedInputSubsystemInterface.AddMappingContext` (pcsubsystem `EnhancedInputLocalPlayerSubsystem` (`GameplayStatics.GetPlayerController` 0)) "/Game/Blueprint/Inputs/IMC_MyCharacter.IMC_MyCharacter" 0 (struct))
  ;;[1 1 1] Affichage du CrossHair
  (bind _returnvalue (`|CreateWidget` "/Game/Blueprint/WBP_Hud.WBP_Hud_C" (`GameplayStatics.GetPlayerController` 0)))
  (`UserWidget.AddToViewport` _returnvalue 0))

(event `EnhancedInput|/Game/Blueprint/Inputs/IA_Sprint`
  (params (ActionValue :type Boolean) (ElapsedSeconds :type "Float (double-precision)") (TriggeredSeconds :type "Float (double-precision)") (InputAction :type "InputAction Object Reference" :default "/Game/Blueprint/Inputs/IA_Sprint.IA_Sprint"))
  (bind _charactermovement (`self.CharacterMovement`))
  ;[1 1 1] Movement
  ;;[1 1 1] IA_Sprint
  (:`Started`
    ;;;[1 1 1] Sprint quand maintient la touche
    (set `CharacterMovementComponent.MaxWalkSpeed` 1200.0 _charactermovement))
  (:`Completed`
    (set `CharacterMovementComponent.MaxWalkSpeed` 600.0 _charactermovement)))

(event `EnhancedInput|/Game/Blueprint/Inputs/IA_Mine`
  (params (ActionValue :type Boolean) (ElapsedSeconds :type "Float (double-precision)") (TriggeredSeconds :type "Float (double-precision)") (InputAction :type "InputAction Object Reference" :default "/Game/Blueprint/Inputs/IA_Mine.IA_Mine"))
  (bind _currentminedblock (`self.currentMinedBlock`))
  ;[1 1 1] IA_Mine
  (:`Started`
    ;;[1 1 1] On récupère l'acteur que l'on vise
    (bind (_returnvalue _outhit) (`self.Recast`))
    (if _returnvalue
      (`self.Cast&DestroyBlock` (`.HitActor` (`GameplayStatics.BreakHitResult` _outhit)))
      ;;[1 1 1] Déclancheur d'event avec un Timer
      (bind _returnvalue_2 (`KismetSystemLibrary.K2_SetTimerDelegate` (delegate `CheckBlock`) 0.25 true))
      (set `self.checkTimer` _returnvalue_2)))
  (:`Completed`
    ;;[1 1 1 1 8] Stop le timer quand arret du minage
    (`self.StopTimer`)
    ;;[1 1 1] On appelle la fonction "StopDestroyBlock" uniquement si le block est valide
    (`/Engine/EditorBlueprintResources/StandardMacros.IsValid` _currentminedblock :!label _label
      (:`Is Valid`
        (`/Game/Blueprint/BP_Block_Parent.StopDestroyBlock` _currentminedblock)))))

(event `CheckBlock`
  ;[1 1 1] IA_Mine
  ;;[1 1 1] On vérifie le block visé
  (`self.CheckBlockAimed`))

(event `StopMining`
  ;[1 1 1] IA_Mine
  ;;[1 1 1] On appelle la fonction "StopDestroyBlock" uniquement si le block est valide
  (goto _label))

(event `EnhancedInput|/Game/Blueprint/Inputs/IA_Jump`
  (params (ActionValue :type Boolean) (ElapsedSeconds :type "Float (double-precision)") (TriggeredSeconds :type "Float (double-precision)") (InputAction :type "InputAction Object Reference" :default "/Game/Blueprint/Inputs/IA_Jump.IA_Jump"))
  ;[1 1 1] Movement
  ;;[1 1 1] IA_Jump
  (:`Started`
    (`self.Jump`))
  (:`Completed`
    (`self.StopJumping`)))

(event `EnhancedInput|/Game/Blueprint/Inputs/IA_Look`
  (params (ActionValue :type "Vector2D Structure") (ElapsedSeconds :type "Float (double-precision)") (TriggeredSeconds :type "Float (double-precision)") (InputAction :type "InputAction Object Reference" :default "/Game/Blueprint/Inputs/IA_Look.IA_Look"))
  ;[1 1 1] Movement
  ;;[1 1 1] IA_Look
  (:`Triggered`
    (`self.AddControllerYawInput` ActionValue_X)
    (`self.AddControllerPitchInput` ActionValue_Y)))

(event `StopTimer`
  ;[1 1 1] IA_Mine
  ;;[1 1 1 1 14] Arret du timer pour casser le block
  (`KismetSystemLibrary.K2_ClearAndInvalidateTimerHandle` (`self.checkTimer`)))

(event `EnhancedInput|/Game/Blueprint/Inputs/IA_PoseAndInterract`
  (params (ActionValue :type Boolean) (ElapsedSeconds :type "Float (double-precision)") (TriggeredSeconds :type "Float (double-precision)") (InputAction :type "InputAction Object Reference" :default "/Game/Blueprint/Inputs/IA_PoseAndInterract.IA_PoseAndInterract"))
  ;[1 1 1] IA_PoseAndInterract
  (:`Started`
    (bind (_returnvalue _outhit) (`self.Recast`))
    (if _returnvalue
      (bind (_bblockinghit _binitialoverlap _time _distance _location _impactpoint _normal _impactnormal _physmat _hitactor) (`GameplayStatics.BreakHitResult` _outhit))
      (bind _asbp_block_interractible_parent (cast `/Game/Blueprint/BP_Block_Interractible_Parent` _hitactor)
        (:`then`
          (`/Game/Blueprint/BP_Block_Interractible_Parent.Interract` _asbp_block_interractible_parent))
        (:`CastFailed`
          ;;[1 1 1 1 14] Spawn du block
          (`|SpawnActorFromClass` (`self.blockToSpawn`) (`KismetMathLibrary.MakeTransform` (`KismetMathLibrary.Vector_SnappedToGrid` (`self.VectorCorrection` _impactpoint _impactnormal) 100.0)) "Undefined" "MultiplyWithRoot" null null))))))

(event `EnhancedInput|/Game/Blueprint/Inputs/IA_ChangeUp`
  (params (ActionValue :type Boolean) (ElapsedSeconds :type "Float (double-precision)") (TriggeredSeconds :type "Float (double-precision)") (InputAction :type "InputAction Object Reference" :default "/Game/Blueprint/Inputs/IA_ChangeUp.IA_ChangeUp"))
  ;[1 1 1 1 17] Changement de block avec la molette de la souris
  (:`Started`
    (`self.ChangeBlockWithWheel` true)))

(event `EnhancedInput|/Game/Blueprint/Inputs/IA_ChangeDown`
  (params (ActionValue :type Boolean) (ElapsedSeconds :type "Float (double-precision)") (TriggeredSeconds :type "Float (double-precision)") (InputAction :type "InputAction Object Reference" :default "/Game/Blueprint/Inputs/IA_ChangeDown.IA_ChangeDown"))
  ;[1 1 1 1 17] Changement de block avec la molette de la souris
  (:`Started`
    (`self.ChangeBlockWithWheel` false)))

(event `EnhancedInput|/Game/Blueprint/Inputs/IA_Switch1`
  (params (ActionValue :type Boolean) (ElapsedSeconds :type "Float (double-precision)") (TriggeredSeconds :type "Float (double-precision)") (InputAction :type "InputAction Object Reference" :default "/Game/Blueprint/Inputs/IA_Switch1.IA_Switch1"))
  (:`Started`
    (set `self.blockToSpawn` "/Game/Blueprint/BP_Block_Parent.BP_Block_Parent_C")))

(event `EnhancedInput|/Game/Blueprint/Inputs/IA_Switch2`
  (params (ActionValue :type Boolean) (ElapsedSeconds :type "Float (double-precision)") (TriggeredSeconds :type "Float (double-precision)") (InputAction :type "InputAction Object Reference" :default "/Game/Blueprint/Inputs/IA_Switch2.IA_Switch2"))
  (:`Started`
    (set `self.blockToSpawn` "/Game/Blueprint/BP_Block_Stone.BP_Block_Stone_C")))

(event `EnhancedInput|/Game/Blueprint/Inputs/IA_Switch3`
  (params (ActionValue :type Boolean) (ElapsedSeconds :type "Float (double-precision)") (TriggeredSeconds :type "Float (double-precision)") (InputAction :type "InputAction Object Reference" :default "/Game/Blueprint/Inputs/IA_Switch3.IA_Switch3"))
  (:`Started`
    (set `self.blockToSpawn` "/Game/Blueprint/BP_Block_Interractible_Glowstone.BP_Block_Interractible_Glowstone_C")))

(event `EnhancedInput|/Game/Blueprint/Inputs/IA_Switch4`
  (params (ActionValue :type Boolean) (ElapsedSeconds :type "Float (double-precision)") (TriggeredSeconds :type "Float (double-precision)") (InputAction :type "InputAction Object Reference" :default "/Game/Blueprint/Inputs/IA_Switch4.IA_Switch4"))
  (:`Started`
    (set `self.blockToSpawn` null)))

(fn `Cast&DestroyBlock`
  (params (block :type "Object Object Reference"))
  ;[1 1 1] On appelle la fonction "DestroyBlock" depuis sa classe et on le set en variable
  (bind _asbp_block_parent (cast `/Game/Blueprint/BP_Block_Parent` block))
  (bind _output_get (set `self.currentMinedBlock` _asbp_block_parent))
  (`/Game/Blueprint/BP_Block_Parent.DestroyBlock` _output_get))

(fn `ChangeBlockWithWheel`
  (params (isUp :type Boolean))
  (bind _returnvalue (+ (`self.blockIndex`) (`KismetMathLibrary.SelectInt` 1 -1 (`local.isUp`))))
  (if (== _returnvalue (`KismetMathLibrary.SelectInt` 4 -1 (`local.isUp`)))
    (set `self.blockIndex` (`KismetMathLibrary.SelectInt` 0 3 (`local.isUp`)))
    (else
      (set `self.blockIndex` _returnvalue)))
  (set `self.blockToSpawn` (select `int` (`self.blockIndex`) :`0` "/Game/Blueprint/BP_Block_Parent.BP_Block_Parent_C" :`1` "/Game/Blueprint/BP_Block_Stone.BP_Block_Stone_C" :`2` "/Game/Blueprint/BP_Block_Interractible_Glowstone.BP_Block_Interractible_Glowstone_C" :`3` null :!type "/Game/Blueprint/BP_Block_Parent Class Reference")))

(fn `CheckBlockAimed`
  (bind (_returnvalue _outhit) (`self.Recast`))
  (if _returnvalue
    (bind (_bblockinghit _binitialoverlap _time _distance _location _impactpoint _normal _impactnormal _physmat _hitactor) (`GameplayStatics.BreakHitResult` _outhit))
    (if (not (== _hitactor (`self.currentMinedBlock`)))
      (`self.StopMining&Reset`)
      (`self.Cast&DestroyBlock` _hitactor))
    (else
      (`self.StopMining&Reset`))))

(fn `Recast`
  (returns (ReturnValue :type Boolean) (OutHit :type "HitResult Structure"))
  (bind _camera (`self.Camera`))
  (bind _returnvalue (`SceneComponent.K2_GetComponentLocation` _camera))
  (bind (_outhit _returnvalue_2) (`KismetSystemLibrary.LineTraceSingleForObjects` :`Start` _returnvalue :`End` (+ _returnvalue (* (`SceneComponent.GetForwardVector` _camera) 500.0)) :`ObjectTypes` (`|MakeArray` "ObjectTypeQuery1" :!type "EObjectTypeQuery Enum") :`DrawDebugType` "ForDuration"))
  (return _returnvalue_2 _outhit))

(fn `SnapCoordCorrection`
  (params (impactPointCoord :type "Float (double-precision)") (impactNormalCoord :type "Float (double-precision)"))
  (returns (ReturnValue :type "Float (double-precision)"))
  (return (+ impactPointCoord (* (`KismetMathLibrary.SelectFloat` -20.0 20.0 (< impactNormalCoord 0.0)) (`KismetMathLibrary.SelectFloat` 0.0 1.0 (== impactNormalCoord 0.0))))))

(fn `StopMining&Reset`
  (`self.StopMining`)
  ;[1 1 1 1 14] Set sans valeur = reset
  (set `self.currentMinedBlock` null))

(fn `UserConstructionScript`)

(fn `VectorCorrection`
  (params (impactPoint :type "Vector Structure") (impactNormal :type "Vector Structure"))
  (returns (correctedVecetor :type "Vector Structure"))
  (return (`KismetMathLibrary.MakeVector` (`self.SnapCoordCorrection` (.x impactPoint) (.x impactNormal)) (`self.SnapCoordCorrection` (.y impactPoint) (.y impactNormal)) (`self.SnapCoordCorrection` (.z impactPoint) (.z impactNormal)))))