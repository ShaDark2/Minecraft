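; Game instance for a Minecraft-style game that keeps the placed blocks of each level in a save game.
; On Init it loads BP_GameSave from the "Save" slot, or creates a new one if none exists.
; SaveBlock and DeleteBlock edit the block array matching the current level name, one for each of two maps.
; Changes stay in memory until SaveAllBlocks writes the slot, which also runs on Shutdown.
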(event `self.ReceiveInit`
  ;[1 1 1 1 10] Se lance à chaque lancement du jeu en tout premier avant tout autre code
  ;[1 1 1] On vérifie si le saveGame existe
  (bind _returnvalue (`GameplayStatics.DoesSaveGameExist` "Save"))
  (if _returnvalue
    ;[1 1 1] On charge la sauvegarde
    (bind _returnvalue_2 (`GameplayStatics.LoadGameFromSlot` "Save"))
    (bind _asbp_game_save (cast `/Game/Blueprint/BP_GameSave` _returnvalue_2))
    (set `self.gameSave` _asbp_game_save)
    (else
      ;[1 1 1] On crée l'objet GameSave dans sa variable
      (bind _returnvalue_3 (`GameplayStatics.CreateSaveGameObject` "/Game/Blueprint/BP_GameSave.BP_GameSave_C"))
      (set `self.gameSave` _returnvalue_3))))

(event `SaveBlock`
  (params (blockToSave :type "/Game/Blueprint/F_SaveBlock Structure"))
  ;[1 1 1] Sauvegarde d'un block dans le level dans lequel on se trouve
  (bind _returnvalue (`GameplayStatics.GetCurrentLevelName` true))
  (switch `string` _returnvalue
    (:`MinecraftMap`
      (`KismetArrayLibrary.Array_AddUnique` (`/Game/Blueprint/BP_GameSave.blocks1` (`self.gameSave`)) blockToSave))
    (:`MinecraftMap2`
      (`KismetArrayLibrary.Array_AddUnique` (`/Game/Blueprint/BP_GameSave.blocks2` (`self.gameSave`)) blockToSave))))

(event `SaveAllBlocks`
  (`GameplayStatics.SaveGameToSlot` (`self.gameSave`) "Save"))

(event `DeleteBlock`
  (params (blockToSave :type "/Game/Blueprint/F_SaveBlock Structure"))
  ;[1 1 1] Retire le block de la save de son level
  (bind _returnvalue (`GameplayStatics.GetCurrentLevelName` true))
  (switch `string` _returnvalue
    (:`MinecraftMap`
      (`KismetArrayLibrary.Array_RemoveItem` (`/Game/Blueprint/BP_GameSave.blocks1` (`self.gameSave`)) blockToSave))
    (:`MinecraftMap2`
      (`KismetArrayLibrary.Array_RemoveItem` (`/Game/Blueprint/BP_GameSave.blocks2` (`self.gameSave`)) blockToSave))))

(event `self.ReceiveShutdown`
  (`self.SaveAllBlocks`))